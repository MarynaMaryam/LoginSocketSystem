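; Player controller for the login screen that shows the login menu and handles server replies to authorization and registration.
; On BeginPlay it creates a LoginMenu widget, passes itself as LoginController and switches input to UI only.
; SocketManager messages are routed by package name, then by their Status field, to print Russian success or error text.
; It only prints these results, with no further action on success.
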(event `self.ReceiveBeginPlay`
  (bind _returnvalue (`|CreateWidget` "/Game/UI/LoginMenu.LoginMenu_C" self self))
  (`UserWidget.AddToPlayerScreen` _returnvalue 0)
  (`WidgetBlueprintLibrary.SetInputMode_UIOnlyEx` self _returnvalue))

(event `self.SocketManager.OnReceiveMessage`
  (params (Package :type "/Game/Blueprints/FModelPackage Structure"))
  (bind _returnvalue (`VaRestJsonObject.GetIntegerField` Package_Data_5_DA8F188543EA40F9247CE1A8A07F6872 "Status"))
  (switch `string` Package_Name_6_9D3E43B3412DA1790BCB9EA8A8DDE206
    (:`Authorization`
      (switch `int` _returnvalue
        (:`0`
          (`KismetSystemLibrary.PrintString` "Авторизация прошла успешно" true true (struct :`G` 1.0 :`A` 1.0) 5.0))
        (:`1`
          (`KismetSystemLibrary.PrintString` "Серверная ошибка" true true (struct :`R` 1.0 :`A` 1.0) 5.0))
        (:`2`
          (`KismetSystemLibrary.PrintString` "Данные введены не верно" true true (struct :`R` 1.0 :`A` 1.0) 5.0))
        (:`3`
          (`KismetSystemLibrary.PrintString` "Пользователь забанен" true true (struct :`R` 1.0 :`A` 1.0) 5.0))))
    (:`Registration`
      (switch `int` _returnvalue
        (:`0`
          (`KismetSystemLibrary.PrintString` "Регистрация прошла успешно" true true (struct :`G` 1.0 :`A` 1.0) 5.0))
        (:`1`
          (`KismetSystemLibrary.PrintString` "Серверная ошибка" true true (struct :`R` 1.0 :`A` 1.0) 5.0))
        (:`2`
          (`KismetSystemLibrary.PrintString` "Пользователь с такими данными уже существует" true true (struct :`R` 1.0 :`A` 1.0) 5.0))
        (:`3`
          (`KismetSystemLibrary.PrintString` "Минимальное кол-во вводимых символов: 4" true true (struct :`R` 1.0 :`A` 1.0) 5.0))))))

(fn `UserConstructionScript`)