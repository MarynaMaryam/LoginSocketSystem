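; SocketManager is the game's client link to a socket server, opening a connection to a hardcoded localhost address on BeginPlay.
; SendPackage encodes a package as JSON Action and Data fields in UTF-8, or reconnects without resending when offline.
; Incoming bytes are decoded, checked for both fields, then forwarded through OnReceiveMessage.
; A disconnect quits the game, and connection status and traffic print to screen.
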(event `self.ReceiveBeginPlay`
  (`self.ConnectToServer`))

(event `ConnectToServer`
  (bind _returnvalue (`LowEntrySocketConnectionLibrary.Connection_Create` "127.0.0.1" 7780 (delegate `OnConnected`) (delegate `OnDisconnected`) (delegate `OnReceivePackage`)))
  (bind _output_get (set `self.SocketConnection` _returnvalue))
  (bind _success (`LowEntrySocketConnection.Connect` _output_get))
  (if (not _success)
    (`KismetSystemLibrary.PrintString` "Возникла ошибка при подлючении к серверу" true true (struct :`R` 1.0 :`A` 1.0) 5.0)))

(event `OnConnected`
  (params (SocketConnection :type "LowEntrySocketConnection Object Reference"))
  (`KismetSystemLibrary.PrintString` "Соединение с сервером установлено" true true (struct :`G` 1.0 :`A` 1.0) 5.0))

(event `OnDisconnected`
  (params (SocketConnection :type "LowEntrySocketConnection Object Reference"))
  (`KismetSystemLibrary.QuitGame` null "Quit"))

(event `OnReceivePackage`
  (params (SocketConnection :type "LowEntrySocketConnection Object Reference") (Bytes :type "Array of Byte (by ref)"))
  (bind (_returnvalue _package) (`self.ReceivePackage` Bytes))
  (if _returnvalue
    (`self.OnReceiveMessage` _package)))

(fn `ReceivePackage`
  (params (Data :type "Array of Byte"))
  (returns (ReturnValue :type Boolean) (Package :type "/Game/Blueprints/FModelPackage Structure"))
  (locals (JsonObject :type "VaRestJsonObject Object Reference"))
  (bind _returnvalue (`LowEntryExtendedStandardLibrary.BytesToStringUtf8` Data))
  (bind _jsonobject (`local.JsonObject`))
  (bind _jsonobject_2 (`local.JsonObject`))
  (set `local.JsonObject` (`VaRestJsonObject.ConstructJsonObject`))
  (`KismetSystemLibrary.PrintString` (`KismetStringLibrary.Concat_StrStr` "Получено: " _returnvalue))
  (bind _returnvalue_2 (`VaRestJsonObject.DecodeJson` _jsonobject _returnvalue))
  (return (and _returnvalue_2 (and (`VaRestJsonObject.HasField` _jsonobject "Action") (`VaRestJsonObject.HasField` _jsonobject "Data"))) (make `/Game/Blueprints/FModelPackage` (`VaRestJsonObject.GetStringField` _jsonobject_2 "Action") (`VaRestJsonObject.GetObjectField` _jsonobject_2 "Data"))))

(fn `SendPackage`
  (params (Package :type "/Game/Blueprints/FModelPackage Structure"))
  (locals (JsonObject :type "VaRestJsonObject Object Reference"))
  (bind _jsonobject (`local.JsonObject`))
  (bind _socketconnection (`self.SocketConnection`))
  (bind _returnvalue (`VaRestJsonObject.EncodeJsonToSingleString` _jsonobject))
  (set `local.JsonObject` (`VaRestJsonObject.ConstructJsonObject`))
  (`VaRestJsonObject.SetStringField` _jsonobject "Action" Package_Name_6_9D3E43B3412DA1790BCB9EA8A8DDE206)
  (`VaRestJsonObject.SetObjectField` _jsonobject "Data" Package_Data_5_DA8F188543EA40F9247CE1A8A07F6872)
  (if (`LowEntrySocketConnection.IsConnected` _socketconnection)
    (`LowEntrySocketConnection.SendMessage` _socketconnection (`LowEntryExtendedStandardLibrary.StringToBytesUtf8` _returnvalue))
    (`KismetSystemLibrary.PrintString` (`KismetStringLibrary.Concat_StrStr` "Отправлено: " _returnvalue))
    (return)
    (else
      (`self.ConnectToServer`)
      (return))))